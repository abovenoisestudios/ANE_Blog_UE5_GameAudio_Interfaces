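; Blueprint-only enemy turret that goes into a timed alert when it receives an AudioInteract event.
; The alert prints a debug message, sets a scalar material parameter on the static mesh and plays an attached sound, if valid, stopped after AlertRefreshTime.
; An OnAlert flag ignores repeat triggers until a delay of the same length zeroes the parameter and clears the alert.
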(event EventBeginPlay)

(event Collision|EventActorBeginOverlap
  (params (OtherActor :type Actor%20Object%20Reference)))

(event EventTick
  (params (DeltaSeconds :type Float%20%28single-precision%29)))

(event EventAudioInteract
  (params (_Instigator :type Actor%20Object%20Reference))
  ;[1 0.63 0.3307] Add a debug message to the screen (Print String)
  ; Set the oscillation parameter on the Static Mesh current material
  ; Play the sound and set it to stop after a set amount of seconds
  (if (not (Variables|EnemyTurretBP|GetbOnAlert))
    (Utilities|FlowControl|Sequence
      (:then_0
        (Variables|EnemyTurretBP|SetbOnAlert true)
        (Development|PrintString (Utilities|String|Append "BP: Audio Interact called on " (Utilities|GetDisplayName self) " by " (Utilities|GetDisplayName _Instigator)) true true "(R=0.000000,G=0.660000,B=1.000000,A=1.000000)" (Variables|EnemyTurretBP|GetAlertRefreshTime)))
      (:then_1
        (Rendering|Material|SetScalarParameterValueonMaterials (Variables|EnemyTurretBP|GetStaticMeshComponent) (Variables|EnemyTurretBP|GetMaterialParamFX) (Variables|EnemyTurretBP|GetMaterialParamOnAlertValue))
        (bind _onalertsound (Variables|EnemyTurretBP|GetOnAlertSound)
          (:then
            (bind _returnvalue (Audio|SpawnSoundAttached _onalertsound (Variables|EnemyTurretBP|GetStaticMeshComponent) "None" "0, 0, 0" "0, 0, 0" "KeepRelativeOffset" false 1.0 1.0 0.0 0 0))
            (Audio|Components|Audio|StopDelayed _returnvalue (Variables|EnemyTurretBP|GetAlertRefreshTime)))
          (:else)))
      (:then_2
        ;[0.5618 0.5053 1] Reset the alert mode after a set amount of seconds
        (Utilities|FlowControl|Delay (Variables|EnemyTurretBP|GetAlertRefreshTime))
        (Rendering|Material|SetScalarParameterValueonMaterials (Variables|EnemyTurretBP|GetStaticMeshComponent) (Variables|EnemyTurretBP|GetMaterialParamFX) 0.0)
        (Variables|EnemyTurretBP|SetbOnAlert false)))))

(fn ConstructionScript)